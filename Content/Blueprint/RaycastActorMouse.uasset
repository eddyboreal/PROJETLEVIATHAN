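; Mouse-driven controller actor that lets the player pick tagged interactable objects and resize or hologram them with keyboard keys.
; A left click line-traces from the cursor and stores the hit interactable in MyGameInstance as the selection.
; P and X grow or shrink it along Y if sizeable.
; H and J toggle hideable objects between overlap-only hologram and solid, blocking states by changing collision and material.
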(event `Key|LeftMouseButton`
  (params (Key :type "Key Structure"))
  (bind (_worldlocation _worlddirection) (`PlayerController.DeprojectMousePositionToWorld` (`GameplayStatics.GetPlayerController` 0)))
  ;[1 1 1] Mouse Raycast
  (:`Pressed`
    (bind _outhit (`KismetSystemLibrary.LineTraceSingle` :`Start` _worldlocation :`End` (+ _worldlocation (* _worlddirection 10000.0)) :`TraceChannel` "TraceTypeQuery1" :`DrawDebugType` "ForDuration"))
    (bind (_bblockinghit _binitialoverlap _time _distance _location _impactpoint _normal _impactnormal _physmat _hitactor) (`GameplayStatics.BreakHitResult` _outhit))
    (if (`self.ActorHasTag` _hitactor "Interactable")
      (cast `/Game/Blueprint/MyInteractableObject` _hitactor
        (:`then`
          (bind _output_get (set `/Game/Blueprint/MyGameInstance.ActorHit` _hitactor (`self.MyGameInstance`)))
          (bind _asinteractable_object (cast `InteractableObject` _output_get)
            (:`then`
              (`KismetSystemLibrary.PrintString` (`InteractableObject.id` _asinteractable_object)))
            (:`CastFailed`
              (`KismetSystemLibrary.PrintString` "failed to cast into interactable obj c++"))))
        (:`CastFailed`
          (`KismetSystemLibrary.PrintString` "cast failed")))
      (else
        (`KismetSystemLibrary.PrintString` "Actor not interactable")
        (set `/Game/Blueprint/MyGameInstance.ActorHit` null (`self.MyGameInstance`))))))

(event `self.ReceiveBeginPlay`
  ;[1 1 1] Get Game Instance
  (set `PlayerController.bShowMouseCursor` true (`GameplayStatics.GetPlayerController` 0))
  (bind _asmy_game_instance (cast `/Game/Blueprint/MyGameInstance` (`GameplayStatics.GetGameInstance`))
    (:`then`
      (set `self.MyGameInstance` _asmy_game_instance))
    (:`CastFailed`
      (`KismetSystemLibrary.PrintString` "cast of game instance at start failed"))))

(event `Key|P`
  (params (Key :type "Key Structure"))
  ;[1 1 1] Resize object
  (:`Pressed`
    (bind _newparam (`self.get Selected actor`))
    (bind _asinteractable_object (cast `InteractableObject` _newparam)
      (:`then`
        (if (`InteractableObject.isSizeable` _asinteractable_object)
          (bind _rootcomponent (`Actor.RootComponent` _newparam))
          (`SceneComponent.SetWorldScale3D` _rootcomponent (+ (0.0 1.0 0.0) (`SceneComponent.K2_GetComponentScale` _rootcomponent)))
          (else
            (`KismetSystemLibrary.PrintString` "object not sizeable" :!label _label))))
      (:`CastFailed`
        (`KismetSystemLibrary.PrintString` "cast failed to interactable object" :!label _label_2)))))

(event `Key|X`
  (params (Key :type "Key Structure"))
  ;[1 1 1] Resize object
  (:`Pressed`
    (bind _newparam (`self.get Selected actor`))
    (bind _asinteractable_object (cast `InteractableObject` _newparam)
      (:`then`
        (if (`InteractableObject.isSizeable` _asinteractable_object)
          (bind _rootcomponent (`Actor.RootComponent` (stale `Key|P` _newparam)))
          (`SceneComponent.SetWorldScale3D` _rootcomponent (- (`SceneComponent.K2_GetComponentScale` _rootcomponent) (0.0 1.0 0.0)))
          (else
            (goto _label))))
      (:`CastFailed`
        (goto _label_2)))))

(event `Key|H`
  (params (Key :type "Key Structure"))
  ;[1 1 1] Hide object
  (:`Pressed`
    (bind _newparam (`self.get Selected actor`))
    (bind _asinteractable_object (cast `InteractableObject` _newparam)
      (:`then`
        (if (`InteractableObject.isHideable` _asinteractable_object)
          (bind _asmy_interactable_object (cast `/Game/Blueprint/MyInteractableObject` _newparam)
            (:`then`
              (set `/Game/Blueprint/MyInteractableObject.isHolographic` true _asmy_interactable_object)
              (`/Game/Blueprint/MyInteractableObject.TurnToHolographic` _asmy_interactable_object "/Game/Sounds/NearHologramSC.NearHologramSC")
              (`PrimitiveComponent.SetCollisionResponseToAllChannels` (`self.GetComponentByClass` _newparam "/Script/Engine.PrimitiveComponent") "ECR_Overlap")
              (`PrimitiveComponent.SetMaterial` (`self.GetComponentByClass` (stale `Key|J` _newparam) "/Script/Engine.StaticMeshComponent") 0 "/Game/VFXMatPack/MaterialInstance/Custom_MI_Hologram1.Custom_MI_Hologram1"))
            (:`CastFailed`
              (`KismetSystemLibrary.PrintString` "cast intcast to my intteractable" :!label _label_3)))
          (else
            (`KismetSystemLibrary.PrintString` "object no hideable" :!label _label_4))))
      (:`CastFailed`
        (goto _label_2)))))

(event `Key|J`
  (params (Key :type "Key Structure"))
  ;[1 1 1] Hide object
  (:`Pressed`
    (bind _newparam (`self.get Selected actor`))
    (bind _asinteractable_object (cast `InteractableObject` _newparam)
      (:`then`
        (if (`InteractableObject.isHideable` _asinteractable_object)
          (bind _asmy_interactable_object (cast `/Game/Blueprint/MyInteractableObject` _newparam)
            (:`then`
              (`PrimitiveComponent.SetCollisionResponseToAllChannels` (`self.GetComponentByClass` _newparam "/Script/Engine.PrimitiveComponent") "ECR_Block")
              (`PrimitiveComponent.SetMaterial` (`self.GetComponentByClass` _newparam "/Script/Engine.StaticMeshComponent") 0 "/Game/Geometry/Meshes/CubeMaterial.CubeMaterial")
              (`/Game/Blueprint/MyInteractableObject.RemoveHolographic` _asmy_interactable_object)
              (set `/Game/Blueprint/MyInteractableObject.isHolographic` false _asmy_interactable_object))
            (:`CastFailed`
              (goto _label_3)))
          (else
            (goto _label_4))))
      (:`CastFailed`
        (goto _label_2)))))

(fn `Cast ActorHit to Interactable object c++`
  (returns (NewParam :type "InteractableObject Object Reference"))
  (bind _asinteractable_object (cast `InteractableObject` (`/Game/Blueprint/MyGameInstance.ActorHit` (`self.MyGameInstance`))))
  (return _asinteractable_object))

(fn `get Selected actor`
  (returns (NewParam :type "Actor Object Reference"))
  (return (`/Game/Blueprint/MyGameInstance.ActorHit` (`self.MyGameInstance`))))

(fn `UserConstructionScript`)