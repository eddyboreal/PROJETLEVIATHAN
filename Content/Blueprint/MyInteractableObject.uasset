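; MyInteractableObject is an interactable actor that plays a sci-fi forcefield hum while overlapped, if flagged as holographic.
; Begin overlap checks IsHolographic and calls TurnToHolographic, which sets the given sound on MyAudioComp and plays it.
; End overlap calls RemoveHolographic, which stops the audio when the same flag is set.
; Despite the event names, only audio changes here, and overlaps are not filtered by actor.
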(event `TurnToHolographic`
  (params (NewParam :type "SoundBase Object Reference"))
  (bind _myaudiocomp (`self.myAudioComp`))
  (`AudioComponent.SetSound` _myaudiocomp NewParam)
  (`AudioComponent.Play` _myaudiocomp 0.0))

(event `RemoveHolographic`
  (if (`self.isHolographic`)
    (`AudioComponent.Stop` (`self.myAudioComp`))))

(event `self.ReceiveActorBeginOverlap`
  (params (OtherActor :type "Actor Object Reference"))
  (if (`self.isHolographic`)
    (`self.TurnToHolographic` "/Game/Sounds/Sound_files/sci-fi_forcefield_hum_loop_03.sci-fi_forcefield_hum_loop_03")))

(event `self.ReceiveActorEndOverlap`
  (params (OtherActor :type "Actor Object Reference"))
  (`self.RemoveHolographic`))

(fn `UserConstructionScript`)